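; BP_Decrease is a destruction-unit Blueprint that shrinks the actor each time it is hit.
; Its Hit event calls the parent handler, then uses a DoN node to capture the original scale on the first hit only.
; Every hit then subtracts a fixed percentage of that starting scale, so shrinking is linear, with no lower clamp or destroy step in this graph.
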(event EventBeginPlay
  (|CallParentFunction) ; This node is disabled and will not be called.\nDrag off pins to build functionality.
)

(event EventTick
  (params (DeltaSeconds :type Float%20%28single-precision%29))
  (|CallParentFunction DeltaSeconds) ; This node is disabled and will not be called.\nDrag off pins to build functionality.
)

(event Collision|EventHit
  (params (MyComp :type Primitive%20Component%20Object%20Reference) (Other :type Actor%20Object%20Reference) (OtherComp :type Primitive%20Component%20Object%20Reference) (bSelfMoved :type Boolean) (HitLocation :type Vector :default "0, 0, 0") (HitNormal :type Vector :default "0, 0, 0") (NormalImpulse :type Vector :default "0, 0, 0") (Hit :type Hit%20Result%20Structure%20%28by%20ref%29))
  (bind _returnvalue (Transformation|GetActorScale3D))
  (|CallParentFunction MyComp Other OtherComp bSelfMoved HitLocation HitNormal NormalImpulse Hit)
  (Utilities|FlowControl|Sequence
    (:then_0
      (Utilities|FlowControl|DoN 1
        (:Exit
          (Variables|Default|SetStarting%20size _returnvalue))))
    (:then_1
      (Transformation|SetActorScale3D (- _returnvalue (* (/ (Variables|Default|GetStarting%20size) "100.000000,100.000000,100.000000") "5.000000,5.000000,5.000000"))))))

(fn ConstructionScript
  (|CallParentFunction))