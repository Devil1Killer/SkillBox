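; Light source actor that blinks its SpotLight in repeating bursts of flashes.
; Tick switches on LampMode into three identical branches, each with its own DoN node.
; A delayed DoN toggles visibility twice per configured flash, while a parallel Delay, built from flash speed, count and repetition frequency, resets it for the next burst.
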(event EventBeginPlay)

(event Collision|EventActorBeginOverlap
  (params (OtherActor :type Actor%20Object%20Reference)))

(event EventTick
  (params (DeltaSeconds :type Float%20%28single-precision%29))
  (switch int (Math|Conversions|ToInteger(Byte) (Variables|Default|GetLamp%20mode))
    (:0
      (Utilities|FlowControl|Sequence
        (:then_0
          (Utilities|FlowControl|Delay (Variables|Default|GetSpeed%20flashes))
          (Utilities|FlowControl|DoN (* (Variables|Default|GetNumber%20flashes) 2) :!label _label
            (:Exit
              (Rendering|ToggleVisibility (Variables|Default|GetSpotLight) false))))
        (:then_1
          (Utilities|FlowControl|Delay (+ (Variables|Default|GetRepetition%20frequency) (* (Variables|Default|GetSpeed%20flashes) (Math|Conversions|ToFloat(Integer) (Variables|Default|GetNumber%20flashes)))))
          (goto _label Reset))))
    (:1
      (Utilities|FlowControl|Sequence
        (:then_0
          (Utilities|FlowControl|Delay (Variables|Default|GetSpeed%20flashes))
          (Utilities|FlowControl|DoN (* (Variables|Default|GetNumber%20flashes) 2) :!label _label_2
            (:Exit
              (Rendering|ToggleVisibility (Variables|Default|GetSpotLight) false))))
        (:then_1
          (Utilities|FlowControl|Delay (+ (Variables|Default|GetRepetition%20frequency) (* (Variables|Default|GetSpeed%20flashes) (Math|Conversions|ToFloat(Integer) (Variables|Default|GetNumber%20flashes)))))
          (goto _label_2 Reset))))
    (:2
      (Utilities|FlowControl|Sequence
        (:then_0
          (Utilities|FlowControl|Delay (Variables|Default|GetSpeed%20flashes))
          (Utilities|FlowControl|DoN (* (Variables|Default|GetNumber%20flashes) 2) :!label _label_3
            (:Exit
              (Rendering|ToggleVisibility (Variables|Default|GetSpotLight) false))))
        (:then_1
          (Utilities|FlowControl|Delay (+ (Variables|Default|GetRepetition%20frequency) (* (Variables|Default|GetSpeed%20flashes) (Math|Conversions|ToFloat(Integer) (Variables|Default|GetNumber%20flashes)))))
          (goto _label_3 Reset))))))

(fn ConstructionScript)