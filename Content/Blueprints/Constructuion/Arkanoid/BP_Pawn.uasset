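; Player pawn for an Arkanoid game that moves left and right and spawns the balls in play.
; Axis input applies a swept world offset each call, without delta-time scaling, and holding Left Shift doubles the step.
; SpawnBall runs on BeginPlay, spawning a BP_Ball at the capsule and decrementing Life.
; It binds a handler to the ball's OnDead event unless Life is 1 before the decrement.
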(event EventBeginPlay
  (CallFunction|SpawnBall))

(event Input|AxisEvents|InputAxisMoveLeftRight
  (params (AxisValue :type Float%20%28single-precision%29))
  (if (< AxisValue 0.0)
    (Transformation|AddActorWorldOffset (Variables|Default|GetLeftSprint) true)))

(event Input|AxisEvents|InputAxisMoveLeftRight
  (params (AxisValue :type Float%20%28single-precision%29))
  (if (> AxisValue 0.0)
    (Transformation|AddActorWorldOffset (Variables|Default|GetRightSprint) true)))

(event Input|KeyboardEvents|LeftShift
  (params (Key :type Key%20Structure :default "None"))
  (bind _right (Variables|Default|GetRight))
  (:Pressed
    (Variables|Default|SetRightSprint (* _right 2.0)))
  (:Released
    (Variables|Default|SetRightSprint _right)))

(event Input|KeyboardEvents|LeftShift
  (params (Key :type Key%20Structure :default "None"))
  (bind _left (Variables|Default|GetLeft))
  (:Pressed
    (Variables|Default|SetLeftSprint (* _left 2.0)))
  (:Released
    (Variables|Default|SetLeftSprint _left)))

(fn ConstructionScript)

(fn SpawnBall
  (bind _returnvalue (Game|SpawnActorfromClass "/Game/Blueprints/Constructuion/BP_Ball.BP_Ball_C" (Math|Transform|MakeTransform (Transformation|GetWorldLocation (Variables|Default|GetCapsule)) "0, 0, 0" "1,1,1") "AlwaysSpawn" 0 0))
  (bind _output_get (Variables|Default|SetPlayingBall _returnvalue))
  (switch int (Math|Conversions|ToInteger(Byte) (Variables|Default|Getlife))
    (:Default
      (EventDispatchers|BindEventtoOnDead _output_get (EventDispatchers|CreateEvent :!event SpawnBall)))
    (:1
      _))
  (Variables|Default|Setlife (- (Variables|Default|Getlife) 1))
  (return))