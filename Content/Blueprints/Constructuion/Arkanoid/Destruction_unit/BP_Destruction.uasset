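; BP_Destruction is a destructible Arkanoid unit that awards score and may drop a bonus.
; Any hit decrements ObjectLife, but only BP_Ball can land the destroying hit.
; On destruction it prints a debug message, adds its Score to the player's BP_Pawn and rolls DropChance.
; A successful roll spawns one of four pickups at the ball's location: protection, extra ball, longer or shorter carriage.
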(event EventBeginPlay)

(event EventTick
  (params (DeltaSeconds :type Float%20%28single-precision%29)))

(event Collision|EventHit
  (params (MyComp :type Primitive%20Component%20Object%20Reference) (Other :type Actor%20Object%20Reference) (OtherComp :type Primitive%20Component%20Object%20Reference) (bSelfMoved :type Boolean) (HitLocation :type Vector :default "0, 0, 0") (HitNormal :type Vector :default "0, 0, 0") (NormalImpulse :type Vector :default "0, 0, 0") (Hit :type Hit%20Result%20Structure%20%28by%20ref%29))
  (bind _rootcomponent (Variables|/Script/Engine.Actor|GetRootComponent Other))
  (bind _returnvalue (Transformation|GetWorldLocation _rootcomponent))
  (bind _returnvalue_2 (Math|Conversions|ToTransform(Vector) _returnvalue))
  (if (<= (Variables|Default|GetObject%20life) 1)
    (Utilities|Casting|CastToBP_Ball Other)
    (Actor|DestroyActor)
    (Development|PrintString "Объект уничтожен" true true "(R=0.067222,G=0.000000,B=1.000000,A=1.000000)" 5.0)
    (Utilities|FlowControl|Sequence
      (:then_0
        (bind _asbp_pawn (Utilities|Casting|CastToBP_Pawn (Game|Player|GetPlayerPawn 0)))
        (Variables|/Game/Blueprints/Constructuion/Arkanoid/BP_Pawn.BP_Pawn_C|SetScore _asbp_pawn (+ (Variables|/Game/Blueprints/Constructuion/Arkanoid/BP_Pawn.BP_Pawn_C|GetScore _asbp_pawn) (Variables|Default|GetScore))))
      (:then_1
        (if (Math|Random|RandomBoolwithWeight (Variables|Default|GetDrop%20Chance))
          (switch int (Math|Random|RandomInteger 4)
            (:0
              (Game|SpawnActorfromClass "/Game/Blueprints/Constructuion/Arkanoid/Bonus/Protection.Protection_C" _returnvalue_2 "AlwaysSpawn" 0 0))
            (:1
              (Game|SpawnActorfromClass "/Game/Blueprints/Constructuion/Arkanoid/Bonus/ExtraBall.ExtraBall_C" _returnvalue_2 "AlwaysSpawn" 0 0))
            (:2
              (Game|SpawnActorfromClass "/Game/Blueprints/Constructuion/Arkanoid/Bonus/IncreaseCarriage.IncreaseCarriage_C" _returnvalue_2 "AlwaysSpawn" 0 0))
            (:3
              (Game|SpawnActorfromClass "/Game/Blueprints/Constructuion/Arkanoid/Bonus/ShortenedCarriage.ShortenedCarriage_C" _returnvalue_2 "AlwaysSpawn" 0 0))))))
    (else
      (Variables|Default|SetObject%20life (- (Variables|Default|GetObject%20life) 1)))))

(fn ConstructionScript)